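; Gameplay ability that dashes the owning character forward.
; It commits, zeroes ground friction, applies a forward velocity-change impulse, sets pawn collision to overlap through the player character helper and plays the Shinbi dash montage.
; Montage completion, blend out or interruption restores the original friction, sets pawn collision to block and ends the ability.
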(event Ability|EventActivateAbility
  (Ability|CommitAbility)
  (bind _ascharacter (Utilities|Casting|CastToCharacter (Ability|GetOwningActorfromActorInfo))
    (:then
      (Variables|Default|SetOriginalGroundFriction (Variables|/Script/Engine.CharacterMovementComponent|GetGroundFriction (Variables|/Script/Engine.Character|GetCharacterMovement _ascharacter)))
      (Variables|/Script/Engine.CharacterMovementComponent|SetGroundFriction (Variables|/Script/Engine.Character|GetCharacterMovement _ascharacter) 0.0)
      (Physics|AddImpulse (Variables|/Script/Engine.Character|GetCharacterMovement _ascharacter) (* (Transformation|GetActorForwardVector _ascharacter) 2e+03) true)
      (bind _characterbase (CallFunction|GetPlayerCharacterandController))
      (Default|SetCollisiontoPawn _characterbase "ECR_Overlap")
      (|PlayMontageandWaitProxy "None" "/Game/BPS/Characters/Animation/AM_Dash_Shinbi.AM_Dash_Shinbi" 1.0 "None" true 1.0
        (:OnCompleted
          _)
        (:OnBlendOut
          _)
        (:OnInterrupted
          _))
      (Variables|/Script/Engine.CharacterMovementComponent|SetGroundFriction (Variables|/Script/Engine.Character|GetCharacterMovement _ascharacter) (Variables|Default|GetOriginalGroundFriction))
      (Default|SetCollisiontoPawn _characterbase "ECR_Block")
      (Ability|EndAbility))
    (:CastFailed
      (Ability|EndAbility))))

(event Ability|EventOnEndAbility
  (params (bWasCancelled :type Boolean)))