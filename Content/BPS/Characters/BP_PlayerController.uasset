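; BP_PlayerController is the player controller that creates the primary UI on BeginPlay and turns player input into pawn actions.
; Movement axes follow the camera's forward and right vectors from its full rotation, while look axes feed controller pitch and yaw.
; Jump casts the pawn to Character, while melee attack and health regen cast to BP_CharacterBase and call its functions, leaving ability logic to the character.
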(event EventBeginPlay
  (bind _returnvalue (UserInterface|CreateWidget "/Game/BPS/UI/WBP_PrimaryUI.WBP_PrimaryUI_C"))
  (bind _output_get (Variables|Default|SetPrimaryUI _returnvalue))
  (UserInterface|Viewport|AddtoViewport _output_get 0))

(event Input|ActionEvents|InputActionJump
  (params (Key :type Key%20Structure))
  ;[1 1 1] Basic Control
  (:Pressed
    (bind _ascharacter (Utilities|Casting|CastToCharacter (Pawn|GetControlledPawn)))
    (Character|Jump _ascharacter)))

(event Input|ActionEvents|InputActionPrimaryAttack
  (params (Key :type Key%20Structure))
  ;[1 1 1] Basic Control
  (:Pressed
    (bind _asbp_character_base (Utilities|Casting|CastToBP_CharacterBase (Pawn|GetControlledPawn)))
    (Default|MeleeAttack _asbp_character_base)))

(event Input|ActionEvents|InputActionHealthRegen
  (params (Key :type Key%20Structure))
  (:Pressed
    (bind _asbp_character_base (Utilities|Casting|CastToBP_CharacterBase (Pawn|GetControlledPawn)))
    (Default|TryHealthRegen _asbp_character_base)))

(event Input|AxisEvents|InputAxisMoveForward
  (params (AxisValue :type Float%20%28single-precision%29))
  ;[1 1 1] Basic Control
  (Pawn|Input|AddMovementInput (Pawn|GetControlledPawn) (Math|Vector|GetForwardVector (Camera|GetCameraRotation (Variables|Default|GetPlayerCameraManager))) AxisValue false))

(event Input|AxisEvents|InputAxisMoveRight
  (params (AxisValue :type Float%20%28single-precision%29))
  ;[1 1 1] Basic Control
  (Pawn|Input|AddMovementInput (Pawn|GetControlledPawn) (Math|Vector|GetRightVector (Camera|GetCameraRotation (Variables|Default|GetPlayerCameraManager))) AxisValue false))

(event Input|AxisEvents|InputAxisLookingUp
  (params (AxisValue :type Float%20%28single-precision%29))
  ;[1 1 1] Basic Control
  (Class|PlayerController|AddPitchInput AxisValue))

(event Input|AxisEvents|InputAxisLookingRight
  (params (AxisValue :type Float%20%28single-precision%29))
  ;[1 1 1] Basic Control
  (Class|PlayerController|AddYawInput AxisValue))

(fn ConstructionScript)