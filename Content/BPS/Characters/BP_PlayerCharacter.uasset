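; BP_PlayerCharacter is the player character Blueprint that keeps the HUD's health and mana globes in step with the character's values.
; OnHealthChanged and OnManaChange each cast the controller to BP_PlayerController and set the matching PrimaryUI glass ball to current divided by maximum.
; The mana event also prints a debug string before the cast.
; BeginPlay, Tick and overlap are disabled stubs, and construction only calls the parent.
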(event EventBeginPlay
  (|CallParentFunction) ; This node is disabled and will not be called.\nDrag off pins to build functionality.
)

(event Collision|EventActorBeginOverlap
  (params (OtherActor :type Actor%20Object%20Reference)))

(event EventTick
  (params (DeltaSeconds :type Float%20%28single-precision%29)))

(event EventOnHealthChanged
  (params (Health :type Float%20%28single-precision%29) (MaxHealth :type Float%20%28single-precision%29))
  (bind _asbp_player_controller (Utilities|Casting|CastToBP_PlayerController (Pawn|GetController)))
  (Default|SetPercentage (Variables|/Game/BPS/UI/WBP_PrimaryUI.WBP_PrimaryUI_C|GetHealthGlassBall (Variables|/Game/BPS/Characters/BP_PlayerController.BP_PlayerController_C|GetPrimaryUI _asbp_player_controller)) (/ Health MaxHealth)))

(event EventOnManaChange
  (params (Mana :type Float%20%28single-precision%29) (MaxMana :type Float%20%28single-precision%29))
  (Development|PrintString "BP_ONMANACHANGE")
  (bind _asbp_player_controller (Utilities|Casting|CastToBP_PlayerController (Pawn|GetController)))
  (Default|SetPercentage (Variables|/Game/BPS/UI/WBP_PrimaryUI.WBP_PrimaryUI_C|GetManaGlassball (Variables|/Game/BPS/Characters/BP_PlayerController.BP_PlayerController_C|GetPrimaryUI _asbp_player_controller)) (/ Mana MaxMana)))

(fn ConstructionScript
  (|CallParentFunction))